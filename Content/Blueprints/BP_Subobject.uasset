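; BP_Subobject is a grid-positioned sub-object that shows its zone type through the color of its static mesh.
; BeginPlay creates a dynamic material instance on the mesh for runtime tinting.
; ConfigSubobjectDisplay sets that material's Color parameter from ObjectZoneType, offsets the mesh by its grid row and column at a fixed height, then unhides it.
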(event EventBeginPlay
  (bind _staticmesh (Variables|Default|GetStaticMesh))
  (|CallParentFunction)
  (bind _returnvalue (Rendering|Material|CreateDynamicMaterialInstance _staticmesh 0 (Rendering|Material|GetMaterial _staticmesh 0) "None" :!class /Script/Engine.PrimitiveComponent))
  (Variables|Components|SetMI_Mat _returnvalue))

(event EventConfigSubobjectDisplay
  (bind _positioningrid (Variables|Default|GetPositionInGrid))
  (bind (_row _column) (Utilities|Struct|BreakPositionInGrid _positioningrid))
  (Rendering|Material|SetVectorParameterValue (Variables|Components|GetMI_Mat) "Color" (Utilities|Select :Index (Variables|Default|GetObjectZoneType) :ZoneNone "" :ZoneI "(R=0.776471,G=0.054902,B=0.050980,A=1.000000)" :ZoneII "(R=0.839216,G=0.666667,B=0.172549,A=1.000000)" :ZoneIII "(R=0.051269,G=0.737911,B=0.063010,A=1.000000)") :!class /Script/Engine.MaterialInstanceDynamic)
  (Transformation|SetRelativeLocation (Variables|Default|GetStaticMesh) (Math|Vector|MakeVector (* _row -2e+02) (* _column 2e+02) -175.0) false false)
  (Development|SetHiddeninGame (Variables|Default|GetStaticMesh) false false))

(fn ConstructionScript)