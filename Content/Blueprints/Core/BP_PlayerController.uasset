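; Player controller that owns the HUD and links its regenerate button to a grid.
; On BeginPlay it creates the W_HUD widget and adds it to the viewport.
; ActivateHUD stores the grid reference and enables the HUD buttons, retrying on a short delay until the widget is valid.
; A regenerate press is forwarded to the stored grid if it is still valid.
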(event Custom|ActivateHUD
  (params (Grid :type BP%20Grid%20Object%20Reference))
  (Variables|Default|SetGrid Grid)
  (bind _w_hud (Variables|Default|GetW_HUD :!label _label)
    (:then
      (Default|ToggleButtons _w_hud true))
    (:else
      (Utilities|FlowControl|Delay 0.25)
      (goto _label))))

(event Custom|OnButtonRegeneratePressed
  (bind _grid (Variables|Default|GetGrid)
    (:then
      (Default|REGENERATE _grid))
    (:else)))

(event EventBeginPlay
  (bind _returnvalue (UserInterface|CreateWidget "/Game/Blueprints/Core/W_HUD.W_HUD_C" self))
  (bind _output_get (Variables|Default|SetW_HUD _returnvalue))
  (UserInterface|Viewport|AddtoViewport _output_get 0))

(fn ConstructionScript)