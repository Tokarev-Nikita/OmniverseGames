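; BP_Grid is a grid actor that generates zoned cells, visualizes them with billboards and activates the player HUD when generation finishes.
; The construction script stores InitializeGrid results in Blueprint variables, which LoadData copies into ZoneData and Cells.
; Visualization events place a zone-specific sprite per cell and a slightly higher billboard for banned cells.
; REGENERATE destroys the banned-cell billboards, then calls RegenerateGrid.
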(event Custom|REGENERATE
  (for _array_element (Variables|Components|GetBannedCells_Billboards)
    (Components|DestroyComponent _array_element))
  (Utilities|Array|Clear (Variables|Components|GetBannedCells_Billboards))
  (Class|OmGGrid|RegenerateGrid))

(event EventBeginPlay
  (|CallParentFunction))

(event EventGenerationFinished
  (bind _asbp_player_controller (Utilities|Casting|CastToBP_PlayerController (Game|GetPlayerController 0)))
  (Default|ActivateHUD _asbp_player_controller self))

(event EventVisualizeCell
  (params (Position :type Position%20in%20Grid%20Structure) (Zone :type EZoneType%20Enum :default "ZoneNone"))
  (bind (_row _column) (Utilities|Struct|BreakPositionInGrid Position))
  (bind _returnvalue (AddComponent|AddBillboardComponent false (Math|Transform|MakeTransform (Math|Vector|MakeVector (* _row -2e+02) (* _column 2e+02) -2e+02) "0, 0, 0" "1,1,1")))
  (Rendering|Components|Sprite|SetSprite _returnvalue (Utilities|Select :Index Zone :ZoneNone "/Game/Assets/S_Zone_None.S_Zone_None" :ZoneI "/Game/Assets/S_Zone_I.S_Zone_I" :ZoneII "/Game/Assets/S_Zone_II.S_Zone_II" :ZoneIII "/Game/Assets/S_Zone_III.S_Zone_III"))
  (Development|SetHiddeninGame _returnvalue (Variables|Default|GetbCellsHiddenInGame) false))

(event EventLoadData
  (Variables|Default|SetZoneData (Variables|Components|GetBP_ZoneData))
  (Variables|Default|SetCells (Variables|Components|GetBP_Cells)))

(event EventVisualizeCellBanning
  (params (Position :type Position%20in%20Grid%20Structure))
  (bind (_row _column) (Utilities|Struct|BreakPositionInGrid Position))
  (bind _returnvalue (AddComponent|AddBillboardComponent false (Math|Transform|MakeTransform (Math|Vector|MakeVector (* _row -2e+02) (* _column 2e+02) -1.9e+02) "0, 0, 0" "1,1,1")))
  (Utilities|Array|Add (Variables|Components|GetBannedCells_Billboards) _returnvalue))

(fn ConstructionScript
  (bind (_zoness _cellss) (Class|OmGGrid|InitializeGrid))
  (Variables|Components|SetBP_ZoneData _zoness)
  (Variables|Components|SetBP_Cells _cellss))